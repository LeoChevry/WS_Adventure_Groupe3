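; Interactable inspectable actor that opens an inspection mode where the player can rotate, pan and zoom a copy of its mesh.
; Construction clones the interactable mesh 1000 units below the actor for a SceneCapture2D that renders only that copy.
; Interact shows the Inspect_UI widget and switches the top-down controller to the inspection input context; exiting restores player input and resets the mesh.
; Zoom adjusts capture FOV, while panning is clamped around the default transform.
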(event `/Game/Blueprints/NewInventory/IInteractInterface.InteractWith`
  (params (PlayerCharacter :type "/Game/TopDown/Blueprints/BP_TopDownCharacter Object Reference")))

(event `/Game/BPInterface/InteractableBPInterface.Interact`
  (params (Character :type "Actor Object Reference"))
  (bind _returnvalue (`GameplayStatics.GetPlayerController` 0))
  (bind _scenecapturecomponent2d (`self.SceneCaptureComponent2D`))
  (`SceneCaptureComponent.SetCaptureSortPriority` _scenecapturecomponent2d 0)
  (`SceneComponent.SetVisibility` _scenecapturecomponent2d true false)
  (`SceneComponent.SetHiddenInGame` (`self.InspectableMesh`) false false)
  (bind _returnvalue_2 (`|CreateWidget` "/Game/Blueprints/Items/Inspect_UI.Inspect_UI_C"))
  (bind _output_get (set `self.InspectUI` _returnvalue_2))
  (`UserWidget.AddToViewport` _output_get 0)
  (set `PlayerController.bShowMouseCursor` true _returnvalue)
  (`WidgetBlueprintLibrary.SetInputMode_GameAndUIEx` _returnvalue null "DoNotLock" false)
  (`MeshComponent.SetOverlayMaterial` (`self.InspectableMesh`) null)
  (bind _asbp_top_down_controller (cast `/Game/TopDown/Blueprints/BP_TopDownController` (`GameplayStatics.GetPlayerController` 0)))
  (`/Game/TopDown/Blueprints/BP_TopDownController.UpdateInput` _asbp_top_down_controller "/Game/TopDown/Input/IMC_Inspection.IMC_Inspection")
  (set `/Game/TopDown/Blueprints/BP_TopDownController.InspectableBP` null _asbp_top_down_controller))

(event `ExitInspectionMode`
  (bind _returnvalue (`GameplayStatics.GetPlayerController` 0))
  ; Exit Inspection Mode
  (`self.ResetInspectableMesh`)
  (`SceneComponent.SetHiddenInGame` (`self.InspectableMesh`) true false)
  (`SceneComponent.SetHiddenInGame` (`self.SceneCaptureComponent2D`) false false)
  (`Widget.RemoveFromParent` (`self.InspectUI`))
  (set `PlayerController.bShowMouseCursor` false _returnvalue)
  (`WidgetBlueprintLibrary.SetInputMode_GameOnly` _returnvalue)
  (bind _asbp_top_down_controller (cast `/Game/TopDown/Blueprints/BP_TopDownController` _returnvalue))
  (`/Game/TopDown/Blueprints/BP_TopDownController.UpdateInput` _asbp_top_down_controller "/Game/TopDown/Input/IMC_Player.IMC_Player"))

(event `ResetInspectableMesh`
  (bind _scenecapturecomponent2d (`self.SceneCaptureComponent2D`))
  ; Exit Inspection Mode
  (`SceneComponent.K2_SetRelativeTransform` (`self.InspectableMesh`) (`self.DefaultPosition`) false false)
  (set `SceneCaptureComponent2D.FOVAngle` 90.0 _scenecapturecomponent2d)
  (`SceneCaptureComponent.SetCaptureSortPriority` _scenecapturecomponent2d 1))

(event `UpdateMeshZoom`
  (params (Axis :type "Float (double-precision)"))
  (set `SceneCaptureComponent2D.FOVAngle` (+ (`SceneCaptureComponent2D.FOVAngle` (`self.SceneCaptureComponent2D`)) (* Axis -3.0)) (`self.SceneCaptureComponent2D`)))

(event `UpdateRotation`
  (params (Vector2D :type "Vector2D Structure"))
  (bind (_x _y) (`KismetMathLibrary.BreakVector2D` Vector2D))
  (bind _inspectablemesh (`self.InspectableMesh`))
  (`SceneComponent.K2_SetRelativeRotation` _inspectablemesh (`KismetMathLibrary.ComposeRotators` (`SceneComponent.RelativeRotation` _inspectablemesh) (`KismetMathLibrary.MakeRotator` (* _y 5.0) 0.0 (* _x -5.0))) false false))

(event `UpdateMeshLocation`
  (params (Vector2D :type "Vector2D Structure"))
  (bind (_x _y) (`KismetMathLibrary.BreakVector2D` Vector2D))
  (bind _inspectablemesh (`self.InspectableMesh`))
  (bind _relativelocation_x (`KismetMathLibrary.BreakVector` (`SceneComponent.RelativeLocation` _inspectablemesh)))
  (bind (_relativelocation_x_2 _relativelocation_y _relativelocation_z) (`KismetMathLibrary.BreakVector` (`SceneComponent.RelativeLocation` (`self.InspectableMesh`))))
  (bind _x_2 (.x (.location (`self.DefaultPosition`))))
  (bind _z (.z (.location (`self.DefaultPosition`))))
  ; Update Mesh Location
  (`SceneComponent.K2_SetRelativeLocation` _inspectablemesh (`KismetMathLibrary.MakeVector` (`KismetMathLibrary.FClamp` (+ _relativelocation_x (* _x 2.0)) (- _x_2 100.0) (+ _x_2 100.0)) 0.0 (`KismetMathLibrary.FClamp` (+ _relativelocation_z (* _y 2.0)) (- _z 100.0) (+ 0.0 _z))) false false))

(fn `UserConstructionScript`
  (bind _inspectablemesh (`self.InspectableMesh`))
  (bind _interactablemesh (`self.InteractableMesh`))
  (bind _inspectablemesh_2 (`self.InspectableMesh`))
  (bind _scenecapturecomponent2d (`self.SceneCaptureComponent2D`))
  (bind (_relativelocation_x _relativelocation_y) (`KismetMathLibrary.BreakVector` (`SceneComponent.RelativeLocation` _scenecapturecomponent2d)))
  (bind (_relativelocation_x_2 _relativelocation_y_2) (`KismetMathLibrary.BreakVector` (`SceneComponent.RelativeLocation` _inspectablemesh_2)))
  (`parent.UserConstructionScript`)
  (`SceneCaptureComponent.ShowOnlyComponent` (`self.SceneCaptureComponent2D`) (`self.InspectableMesh`))
  (`StaticMeshComponent.SetStaticMesh` _inspectablemesh (`StaticMeshComponent.StaticMesh` _interactablemesh))
  (`SceneComponent.K2_SetRelativeTransform` _inspectablemesh (`SceneComponent.GetRelativeTransform` _interactablemesh) false false)
  (`SceneComponent.K2_SetRelativeLocation` _inspectablemesh_2 (`KismetMathLibrary.MakeVector` _relativelocation_x_2 _relativelocation_y_2 -1000.0) false false)
  (`SceneComponent.K2_SetRelativeLocation` _scenecapturecomponent2d (`KismetMathLibrary.MakeVector` _relativelocation_x _relativelocation_y -1000.0) false false)
  (set `self.DefaultPosition` (`SceneComponent.GetRelativeTransform` (`self.InspectableMesh`))))