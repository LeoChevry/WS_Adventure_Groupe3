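; Test item Blueprint that responds to Interact and Inspect events inherited from a parent class or interface.
; Interact runs the parent Interact logic, then destroys the actor, so the item is single-use.
; Inspect also calls the parent Interact rather than a parent Inspect, but leaves the actor in place.
; BeginPlay, overlap and Tick are disabled stubs, and the construction script only calls its parent.
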(event `/Game/BPInterface/InteractableBPInterface.Interact`
  (params (Character :type "Actor Object Reference"))
  (`parent.Interact` null)
  (`self.K2_DestroyActor`))

(event `/Game/BPInterface/InteractableBPInterface.Inspect`
  (params (Character :type "Actor Object Reference"))
  (`parent.Interact` null))

(fn `UserConstructionScript`
  (`parent.UserConstructionScript`))