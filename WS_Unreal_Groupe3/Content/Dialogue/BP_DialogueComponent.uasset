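; Dialogue component that shows data table driven conversations in a WPI_Dialogue widget.
; Each row supplies the text, the next row and table, and an end flag, so conversations chain across tables.
; InteractDialogue clears its widget reference before branching to close, update or create, adding WB_Options buttons for open-ended rows on creation.
; OptionSelected clears the options and shows the chosen row; LeaveDialogue removes the widget.
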(event `/Game/Dialogue/BP_Interact.LeaveDialogue`
  (`/Engine/EditorBlueprintResources/StandardMacros.IsValid` (`self.DialogueWidget`)
    (:`Is Valid`
      (`Widget.RemoveFromParent` (`self.DialogueWidget`) :!label _label)
      (set `self.EndDialogue` false))))

(event `OptionSelected`
  (params (RowName :type Name) (DataTable :type "DataTable Object Reference"))
  (bind _dialoguewidget (`self.DialogueWidget`))
  (bind _returnvalue (`|GetDataTableRow` DataTable RowName)
    (:`then`
      (`PanelWidget.ClearChildren` (`/Game/Dialogue/WPI_Dialogue.OptionScrollBox` _dialoguewidget))
      (bind (_dialogue _row _datatable _enddialogue) (break `/Game/Dialogue/Dialogue_Structure` _returnvalue))
      (`/Game/Dialogue/WPI_Dialogue.Update Dialogue` _dialoguewidget _dialogue)
      (set `self.Row Name` _row)
      (set `self.Data Table` _datatable)
      (set `self.EndDialogue` _enddialogue))))

(event `/Game/Dialogue/BP_Interact.InteractDialogue`
  (params (PlayerRef :type "/Game/TopDown/Blueprints/BP_TopDownCharacter Object Reference"))
  (set `self.DialogueWidget` null)
  (if (`self.EndDialogue`)
    (goto _label)
    (else
      (`/Engine/EditorBlueprintResources/StandardMacros.IsValid` (`self.DialogueWidget`)
        (:`Is Valid`
          (bind _returnvalue (`|GetDataTableRow` (`self.Data Table`) (`self.Row Name`))
            (:`then`
              (bind (_dialogue _row _datatable _enddialogue) (break `/Game/Dialogue/Dialogue_Structure` _returnvalue))
              (`/Game/Dialogue/WPI_Dialogue.Update Dialogue` (`self.DialogueWidget`) _dialogue)
              (set `self.Row Name` _row)
              (set `self.Data Table` _datatable)
              (set `self.EndDialogue` _enddialogue))))
        (:`Is Not Valid`
          (bind _returnvalue_2 (`|GetDataTableRow` (`self.Data Table`) (`self.Row Name`))
            (:`then`
              (bind (_dialogue_2 _row_2 _datatable_2 _enddialogue_2 _openendeddialogue_ _opendialogueoption) (break `/Game/Dialogue/Dialogue_Structure` _returnvalue_2))
              (bind _returnvalue_3 (`|CreateWidget` "/Game/Dialogue/WPI_Dialogue.WPI_Dialogue_C" null (`KismetTextLibrary.Conv_NameToText` (`self.Name`)) _dialogue_2))
              (bind _output_get (set `self.DialogueWidget` _returnvalue_3))
              (`UserWidget.AddToViewport` _output_get 0)
              (set `self.Row Name` _row_2)
              (set `self.Data Table` _datatable_2)
              (set `self.EndDialogue` _enddialogue_2)
              (if _openendeddialogue_
                (for _array_element _opendialogueoption
                  (bind (_optionname _row_3 _datatable_3) (break `/Game/Dialogue/OptionsDialogue_Structure` _array_element))
                  (bind _returnvalue_4 (`|CreateWidget` "/Game/Dialogue/WB_Options.WB_Options_C" null (`KismetTextLibrary.Conv_NameToText` _optionname) self _row_3 _datatable_3))
                  (`PanelWidget.AddChild` (`/Game/Dialogue/WPI_Dialogue.OptionScrollBox` (`self.DialogueWidget`)) _returnvalue_4))))
            (:`RowNotFound`
              (`KismetSystemLibrary.PrintString` "Row not Found"))))))))