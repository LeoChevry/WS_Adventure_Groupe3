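; Interaction component that finds objects tagged Interactable in front of the player character and lets the owner interact with them.
; An overlap counter starts a looping timer for sphere traces from the character mesh, though the stop branch clears it only if the handle is already invalid.
; Trace results set the current target and send hover/unhover messages.
; IA_Interact sends that target an interact message with the owner.
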(event `On Interactable Overlap`
  (params (Overlap :type Boolean))
  (`|ExecutionSequence`
    (:`then_0`
      (bind _output_get (set `self.Overlap Count` (+ (`self.Overlap Count`) (select `bool` Overlap :`false` -1 :`true` 1))))
      (`KismetSystemLibrary.PrintString` (`KismetStringLibrary.Conv_IntToString` _output_get)))
    (:`then_1`
      (`self.Draw Trace` (> (`self.Overlap Count`) 0)))))

(event `Draw Trace`
  (params (`Draw Trace` :type Boolean))
  (bind _returnvalue (not (`KismetSystemLibrary.K2_IsValidTimerHandle` (`self.Trace Timer`))))
  (if `Draw Trace`
    (if _returnvalue
      (bind _returnvalue_2 (`KismetSystemLibrary.K2_SetTimer` null "DetectSight" 0.1 true))
      (set `self.Trace Timer` _returnvalue_2))
    (elif _returnvalue
      (`KismetSystemLibrary.K2_ClearAndInvalidateTimerHandle` (`self.Trace Timer`))
      (bind _interactalbe_object (`self.Interactalbe Object`)
        (:`then`
          (message `/Game/BPInterface/InteractableBPInterface.On UnHovered` _interactalbe_object)
          (set `self.Interactalbe Object` null)
          (set `self.CanInteract` false))
        (:`else`)))))

(event `EnhancedInput|/Game/TopDown/Input/IA_Interact`
  (params (ActionValue :type Boolean) (ElapsedSeconds :type "Float (double-precision)") (TriggeredSeconds :type "Float (double-precision)") (InputAction :type "InputAction Object Reference" :default "/Game/TopDown/Input/IA_Interact.IA_Interact"))
  (:`Started`
    (if (`self.CanInteract`)
      (message `/Game/BPInterface/InteractableBPInterface.Interact` (`self.Interactalbe Object`) (`self.GetOwner`)))))

(event `DetectSight`
  (bind _mesh (`Character.Mesh` (`GameplayStatics.GetPlayerCharacter` 0)))
  (bind _returnvalue (`SceneComponent.K2_GetComponentLocation` _mesh))
  ; Fait un rayon (raycast) de collision, a partir de ou est l'écran, faut le faire sur le mesh du perso
  (bind (_outhit _returnvalue_2) (`KismetSystemLibrary.SphereTraceSingle` :`Start` (+ _returnvalue (0.0 0.0 75.0)) :`End` (+ (+ (* (`KismetMathLibrary.RotateAngleAxis` (`SceneComponent.GetForwardVector` _mesh) 90.0 (`SceneComponent.GetUpVector` _mesh)) 100.0) _returnvalue) (0.0 0.0 75.0)) :`Radius` 75.0 :`TraceChannel` "TraceTypeQuery1" :`DrawDebugType` "ForDuration" :`DrawTime` 0.1))
  (if _returnvalue_2
    (bind (_bblockinghit _binitialoverlap _time _distance _location _impactpoint _normal _impactnormal _physmat _hitactor) (`GameplayStatics.BreakHitResult` _outhit))
    (if (`Actor.ActorHasTag` _hitactor "Interactable")
      (if (not (== _hitactor (`self.Interactalbe Object`)))
        (bind _interactalbe_object (`self.Interactalbe Object`)
          (:`then`
            (message `/Game/BPInterface/InteractableBPInterface.On UnHovered` _interactalbe_object))
          (:`else`
            _))
        (set `self.Interactalbe Object` _hitactor)
        (set `self.CanInteract` true)
        (message `/Game/BPInterface/InteractableBPInterface.On Hovered` (`self.Interactalbe Object`))
        (`KismetSystemLibrary.PrintString` "Looking"))
      (else
        (if (`self.CanInteract`) :!label _label
          (bind _interactalbe_object_2 (`self.Interactalbe Object`)
            (:`then`
              (message `/Game/BPInterface/InteractableBPInterface.On UnHovered` _interactalbe_object_2)
              (set `self.Interactalbe Object` null)
              (set `self.CanInteract` false)
              (`KismetSystemLibrary.PrintString` "Not Looking"))
            (:`else`)))))
    (else
      (goto _label))))