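; Base interactable actor that signals the player when in range and highlights itself when hovered.
; A sphere trigger reports player overlap begin and end through the InteractionComponent's OnInteractableOverlap.
; Hover events toggle the tooltip, a highlight overlay material on the mesh and custom depth stencil for outlining, with the overlay cleared on BeginPlay and unhover.
; Interact is a placeholder that only prints a debug string.
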(event `self.Sphere.OnComponentBeginOverlap`
  (params (OverlappedComponent :type "PrimitiveComponent Object Reference") (OtherActor :type "Actor Object Reference") (OtherComp :type "PrimitiveComponent Object Reference") (OtherBodyIndex :type Integer) (bFromSweep :type Boolean) (SweepResult :type "HitResult Structure (by ref)"))
  (bind _returnvalue (`self.GetComponentByClass` OtherActor "/Game/Blueprints/InteractionComponent.InteractionComponent_C"))
  (if (== OtherActor (`GameplayStatics.GetPlayerCharacter` 0))
    (if (`KismetSystemLibrary.IsValid` _returnvalue)
      (`/Game/Blueprints/InteractionComponent.On Interactable Overlap` _returnvalue true))))

(event `self.Sphere.OnComponentEndOverlap`
  (params (OverlappedComponent :type "PrimitiveComponent Object Reference") (OtherActor :type "Actor Object Reference") (OtherComp :type "PrimitiveComponent Object Reference") (OtherBodyIndex :type Integer))
  (bind _returnvalue (`self.GetComponentByClass` "/Game/Blueprints/InteractionComponent.InteractionComponent_C"))
  (if (== null (`GameplayStatics.GetPlayerCharacter` 0))
    (if (`KismetSystemLibrary.IsValid` _returnvalue)
      (`/Game/Blueprints/InteractionComponent.On Interactable Overlap` _returnvalue false))))

(event `self.ReceiveBeginPlay`
  (`MeshComponent.SetOverlayMaterial` (`self.InteractableMesh`) null :!label _label))

(event `/Game/BPInterface/InteractableBPInterface.On Hovered`
  (`SceneComponent.SetVisibility` (`self.ToolTip_UI`) true false)
  (`self.Highlight Outline` true)
  (`MeshComponent.SetOverlayMaterial` (`self.InteractableMesh`) "/Game/UI/MI_Highlight.MI_Highlight"))

(event `/Game/BPInterface/InteractableBPInterface.On UnHovered`
  (`SceneComponent.SetVisibility` (`self.ToolTip_UI`) false false)
  (`self.Highlight Outline` false)
  (goto _label))

(event `Highlight Outline`
  (params (Show :type Boolean))
  (bind _interactablemesh (`self.InteractableMesh`))
  ; Event Highlight
  (`PrimitiveComponent.SetRenderCustomDepth` _interactablemesh Show)
  (`PrimitiveComponent.SetCustomDepthStencilValue` _interactablemesh (select `bool` Show :`true` 1)))

(event `/Game/BPInterface/InteractableBPInterface.Interact`
  (params (Character :type "Actor Object Reference"))
  (`KismetSystemLibrary.PrintString` "Interact"))

(fn `UserConstructionScript`)