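; ItemDataComponent is an actor component that makes its owner a pickup item for the player's inventory.
; On begin play it turns on replication for the owning actor.
; Interacting passes the ItemID row name and Quantity to the player character's InventorySystem, then destroys the owner if the add succeeds.
; LookAt currently returns an empty string.
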(event `self.ReceiveBeginPlay`
  (`Actor.SetReplicates` (`self.GetOwner`) true))

(event `/Game/Blueprints/NewInventory/IInteractInterface.InteractWith`
  (params (PlayerCharacter :type "/Game/TopDown/Blueprints/BP_TopDownCharacter Object Reference"))
  (bind _inventory_system (`/Game/TopDown/Blueprints/BP_TopDownCharacter.Inventory_System` PlayerCharacter))
  (bind (_itemid_datatable _itemid_rowname) (break `DataTableRowHandle` (`self.ItemID`)))
  (`/Engine/EditorBlueprintResources/StandardMacros.IsValid` _inventory_system
    (:`Is Valid`
      (bind _success (`/Game/Blueprints/NewInventory/Inventory_System.AddToInventory` _inventory_system _itemid_rowname (`self.Quantity`)))
      (if _success
        (`Actor.K2_DestroyActor` (`self.GetOwner`))))))

(fn `LookAt`
  (returns (Message :type Text))
  (return ""))